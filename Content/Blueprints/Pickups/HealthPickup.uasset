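; HealthPickup is a pickup actor that restores health to the player character on overlap.
; When an overlapping actor casts to FPS_Character, it adds its Health amount, plays a 2D pickup sound and destroys itself.
; Tick spins the health mesh around yaw, scaling RotationRate by delta time for frame-rate-independent rotation.
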(event `self.ReceiveActorBeginOverlap`
  (params (OtherActor :type "Actor Object Reference"))
  (bind _asfps_character (cast `/Game/Blueprints/Character/FPS_Character` OtherActor))
  (`/Game/Blueprints/Character/FPS_Character.AddHealth` _asfps_character (`self.Health`))
  (`GameplayStatics.PlaySound2D` "/Game/Assets/Sounds/Health/sw_Pickup_Health.sw_Pickup_Health" 1.0 1.0 0.0 null null)
  (`self.K2_DestroyActor`))

(event `self.ReceiveTick`
  (params (DeltaSeconds :type "Float (single-precision)"))
  (`SceneComponent.K2_AddWorldRotation` (`self.HealthMesh`) (`KismetMathLibrary.MakeRotator` 0.0 0.0 (* DeltaSeconds (`self.RotationRate`))) false false))

(fn `UserConstructionScript`)