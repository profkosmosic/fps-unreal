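; Ammo pickup actor that gives ammo to the player's FPS_Character when it overlaps the pickup.
; On overlap it adds its Ammo amount to the character, plays an equip sound and destroys itself.
; Tick spins the ammo mesh around yaw at RotationRate, scaled by delta time for frame-rate independence.
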(event `self.ReceiveActorBeginOverlap`
  (params (OtherActor :type "Actor Object Reference"))
  (bind _asfps_character (cast `/Game/Blueprints/Character/FPS_Character` OtherActor))
  (`/Game/Blueprints/Character/FPS_Character.AddAmmo` _asfps_character (`self.Ammo`))
  (`GameplayStatics.PlaySound2D` "/Game/Assets/Sounds/Ammo/sw_AmmoEquip.sw_AmmoEquip" 1.0 1.0 0.0 null null)
  (`self.K2_DestroyActor`))

(event `self.ReceiveTick`
  (params (DeltaSeconds :type "Float (single-precision)"))
  (`SceneComponent.K2_AddWorldRotation` (`self.AmmoMesh`) (`KismetMathLibrary.MakeRotator` 0.0 0.0 (* DeltaSeconds (`self.RotationRate`))) false false))

(fn `UserConstructionScript`)